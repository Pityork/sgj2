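; BP_NPC is an NPC character with a health pool that is destroyed when its health reaches zero or below.
; AnyDamage subtracts incoming damage from HealthPoint without audio feedback.
; A separate CustomEvent applies the same logic but plays a hit sound at the actor's location, plus a death sound before destroying it.
; SetWalkspeed sets the movement component's maximum walk speed.
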(event `self.ReceiveAnyDamage`
  (params (Damage :type "Float (single-precision)") (DamageType :type "DamageType Object Reference") (InstigatedBy :type "Controller Object Reference") (DamageCauser :type "Actor Object Reference"))
  (bind _output_get (set `self.health_point` (- (`self.health_point`) (`KismetMathLibrary.Conv_DoubleToInt64` Damage))))
  (if (<= _output_get 0)
    (`self.K2_DestroyActor` self)))

(event `CustomEvent`
  (params (Damage :type "Float (single-precision)") (DamageType :type "DamageType Object Reference") (InstigatedBy :type "Controller Object Reference") (DamageCauser :type "Actor Object Reference"))
  ; dzwiekj ziutek uderzony
  (bind _output_get (set `self.health_point` (- (`self.health_point`) (`KismetMathLibrary.Conv_DoubleToInt64` Damage))))
  (`GameplayStatics.PlaySoundAtLocation` null (`self.K2_GetActorLocation`) (struct) 1.0 1.0 0.0 null null null null)
  ;; dzwiek ziutek martwy
  (if (<= _output_get 0)
    (`GameplayStatics.PlaySoundAtLocation` null (`self.K2_GetActorLocation`) (struct) 1.0 1.0 0.0 null null null null)
    (`self.K2_DestroyActor` self)))

(fn `SetWalkspeed`
  (params (Speed :type "Float (double-precision)"))
  (set `CharacterMovementComponent.MaxWalkSpeed` Speed (`self.CharacterMovement`)))

(fn `UserConstructionScript`)