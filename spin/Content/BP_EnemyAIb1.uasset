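; Enemy AI Blueprint for a melee attacker (police skeleton animations) that damages the player and can be killed by them.
; Sphere overlap with the player enables Fight, so Tick attacks whenever the HitFrequency cooldown allows; player collision jumps into the same attack.
; Attacks alternate two animations and damage the Hit event's Other actor, then restore the default animation.
; Only player-caused damage lowers health, playing sounds on hit and death before destroying the actor.
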(event `self.ReceiveAnyDamage`
  (params (Damage :type "Float (single-precision)") (DamageType :type "DamageType Object Reference") (InstigatedBy :type "Controller Object Reference") (DamageCauser :type "Actor Object Reference"))
  (if (== DamageCauser (`GameplayStatics.GetPlayerCharacter` 0))
    ; dzwiekj ziutek uderzony
    (bind _output_get (set `self.health_points` (- (`self.health_points`) (`KismetMathLibrary.Conv_DoubleToInt64` Damage))))
    (`GameplayStatics.PlaySoundAtLocation` null (`self.K2_GetActorLocation`) (struct) 1.0 1.0 0.0 null null null null)
    ;; dzwiek ziutek martwy
    (if (<= _output_get 0)
      (`GameplayStatics.PlaySoundAtLocation` null (`self.K2_GetActorLocation`) (struct) 1.0 1.0 0.0 null null null null)
      (`self.K2_DestroyActor` self))))

(event `self.ReceiveTick`
  (params (DeltaSeconds :type "Float (single-precision)"))
  (bind _mesh (`self.Mesh`))
  (`|ExecutionSequence`
    (:`then_0`
      (if (`self.can_hit`)
        _
        (elif (not (`self.hit_timer_started`))
          (set `self.hit_timer_started` true)
          (`KismetSystemLibrary.Delay` (/ 1.0 (`self.hit_frequency`)))
          (set `self.can_hit` true)
          (set `self.hit_timer_started` false))))
    (:`then_1`
      (if (`self.Fight?`)
        (if (`self.can_hit`) :!label _label
          (`/Engine/EditorBlueprintResources/StandardMacros.FlipFlop`
            (:`A`
              (`SkeletalMeshComponent.PlayAnimation` _mesh "/Game/Modele/Police_Skeleton_gotowydopierdolniecia.Police_Skeleton_gotowydopierdolniecia" false))
            (:`B`
              (`SkeletalMeshComponent.PlayAnimation` _mesh "/Game/Modele/Police_Skeleton_juzzajebal.Police_Skeleton_juzzajebal" false)))
          (`GameplayStatics.ApplyDamage` (stale `self.ReceiveHit` Other) (`KismetMathLibrary.Conv_Int64ToDouble` (`self.damage`)) null self)
          (set `self.can_hit` false)
          (`KismetSystemLibrary.Delay` 0.333333)
          (`SkeletalMeshComponent.SetAnimation` (`self.Mesh`) "/Game/Modele/Police_Skeleton_Sequence1.Police_Skeleton_Sequence1"))))))

(event `self.ReceiveHit`
  (params (MyComp :type "PrimitiveComponent Object Reference") (Other :type "Actor Object Reference") (OtherComp :type "PrimitiveComponent Object Reference") (bSelfMoved :type Boolean) (HitLocation :type "Vector Structure") (HitNormal :type "Vector Structure") (NormalImpulse :type "Vector Structure") (Hit :type "HitResult Structure (by ref)"))
  (if (== (`GameplayStatics.GetPlayerCharacter` 0) Other)
    (goto _label)))

(event `self.Sphere.OnComponentBeginOverlap`
  (params (OverlappedComponent :type "PrimitiveComponent Object Reference") (OtherActor :type "Actor Object Reference") (OtherComp :type "PrimitiveComponent Object Reference") (OtherBodyIndex :type Integer) (bFromSweep :type Boolean) (SweepResult :type "HitResult Structure (by ref)"))
  (if (== OtherActor (`GameplayStatics.GetPlayerCharacter` 0))
    (set `self.Fight?` true)))

(event `self.Sphere.OnComponentEndOverlap`
  (params (OverlappedComponent :type "PrimitiveComponent Object Reference") (OtherActor :type "Actor Object Reference") (OtherComp :type "PrimitiveComponent Object Reference") (OtherBodyIndex :type Integer))
  (if (== OtherActor (`GameplayStatics.GetPlayerCharacter` 0))
    (set `self.Fight?` false)))

(fn `UserConstructionScript`)